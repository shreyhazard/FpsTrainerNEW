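; BP_weaponBase is a base weapon Blueprint that handles magazine ammo, firing and timed reloading.
; FireWeapon spends a round, spawns muzzle particles and sound at an Arrow component, then calls WeaponTrace, an empty event apparently left for child weapons.
; An empty magazine triggers an automatic reload, which shares a DoOnce with manual Reload to block overlaps.
; Reloading shows an animated WB_ReloadBar widget, refilling ammo after ReloadTime.
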(event Custom|ReloadWeapon
  ;[1 1 1] rELOAD
  (Utilities|FlowControl|DoOnce false :!label _label
    (:Completed
      (bind _returnvalue (UserInterface|CreateWidget "/Game/Blueprints/Weapons/WB_ReloadBar.WB_ReloadBar_C"))
      (Default|ReloadAnimation _returnvalue (Variables|Ammo|GetreloadTime))
      (UserInterface|Viewport|AddtoViewport _returnvalue 0)
      (Utilities|FlowControl|Delay (Variables|Ammo|GetreloadTime))
      (Variables|Ammo|SetAmmo (Variables|Ammo|GetMaxMagzineAmmo))
      (goto _label Reset))))

(event Custom|WeaponTrace)

(event EventReload
  ;[1 1 1] rELOAD
  (Utilities|FlowControl|DoOnce false :!label _label
    (:Completed
      (bind _returnvalue (UserInterface|CreateWidget "/Game/Blueprints/Weapons/WB_ReloadBar.WB_ReloadBar_C"))
      (Default|ReloadAnimation _returnvalue (Variables|Ammo|GetreloadTime))
      (UserInterface|Viewport|AddtoViewport _returnvalue 0)
      (Utilities|FlowControl|Delay (Variables|Ammo|GetreloadTime))
      (Variables|Ammo|SetAmmo (Variables|Ammo|GetMaxMagzineAmmo))
      (goto _label Reset))))

(event EventFireWeapon
  ;[1 1 1] FireWeapon
  (Utilities|Int<=Int (Variables|Ammo|GetAmmo)
    (:True
      (CallFunction|ReloadWeapon))
    (:False
      (Variables|Ammo|SetAmmo (- (Variables|Ammo|GetAmmo) 1))
      (CallFunction|WeaponFireEffects)
      (CallFunction|WeaponTrace)
      (Utilities|Int<=Int (Variables|Ammo|GetAmmo)
        (:True
          (CallFunction|ReloadWeapon))))))

(event EventBeginPlay
  (Variables|Ammo|SetAmmo (Variables|Ammo|GetMaxMagzineAmmo)))

(fn ConstructionScript)

(fn WeaponFireEffects
  (bind _arrow (Variables|Default|GetArrow))
  (bind _returnvalue (Transformation|GetWorldTransform _arrow))
  (Effects|SpawnEmitteratLocation (Variables|WeaponFireEffects|GetWeapon%20Emitter%20Template) (.location _returnvalue) (.rotation _returnvalue) (Variables|WeaponFireEffects|GetWeapon%20Fire%20Emmiter%20Scale))
  (Audio|SpawnSoundatLocation (Variables|WeaponFireEffects|GetWeapon%20Fire%20Sound) (.location _returnvalue) "0, 0, 0" 1.0 1.0 0.0 0 0)
  (return))

(fn GetFOVmultiplier
  (return (Variables|Default|GetFOVmultiplier)))